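; Floor actor that builds a rectangular tiled floor from Columns, Rows and TileSize.
; The Construction Script computes start and end bounds centred on the actor's origin, then adds one Floor mesh instance per grid cell.
; A single flat loop derives each tile's column and row with modulo and integer division, counting tiles as it goes.
; The event graph holds no active logic.
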(fn `UserConstructionScript`
  (locals (XOffset :type Integer :default 0))
  (bind _columns (`self.Columns`))
  (bind _tilesize (`self.TileSize`))
  (bind _tilesize_2 (`self.TileSize`))
  (bind _returnvalue (* (`self.Rows`) _tilesize))
  (bind _returnvalue_2 (* (`self.Columns`) (`self.Rows`)))
  (bind _returnvalue_3 (* (`self.Columns`) _tilesize))
  (bind _returnvalue_4 (- 0 (/ _returnvalue 2)))
  (bind _returnvalue_5 (- 0 (/ _returnvalue_3 2)))
  (`|ExecutionSequence`
    (:`then_0`
      ;[1 1 1] Initialize Helper Variables
      (set `self.XStart` _returnvalue_5)
      (set `self.YStart` _returnvalue_4)
      (set `self.XEnd` (+ _returnvalue_3 _returnvalue_5))
      (set `self.YEnd` (+ _returnvalue _returnvalue_4))
      (set `self.TilesGenerated` 0))
    (:`then_1`
      ;[1 1 1] Create Floor Tiles
      (set `self.ColumnsTimesRows` _returnvalue_2))
    (:`then_2`
      (for _index (range _returnvalue_2)
        (`InstancedStaticMeshComponent.AddInstance` (`self.Floor`) (`KismetMathLibrary.Conv_VectorToTransform` (`KismetMathLibrary.MakeVector` (`KismetMathLibrary.Conv_IntToDouble` (+ (* (mod _index _columns) _tilesize_2) (`self.XStart`))) (`KismetMathLibrary.Conv_IntToDouble` (+ (`self.YStart`) (* (/ _index _columns) _tilesize_2))))))
        (bind _result (`/Engine/EditorBlueprintResources/StandardMacros.IncrementInt` (`self.TilesGenerated`))
          (:`  `
            (set `self.TilesGenerated` _result)))))))